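; NPC AI controller that runs guard behavior and tracks perceived targets.
; On BeginPlay it loads the PatrolData blackboard and starts the GuardBehaviour behavior tree.
; Perception updates write sensed actors without the "Enemy" tag to the blackboard's enemy key, clearing it when such an actor is no longer sensed.
; FindPatrolRoute is an empty stub.
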(event `self.ReceiveBeginPlay`
  (`KismetSystemLibrary.PrintString` "NPC AI Reporting for duty")
  (bind _blackboardcomponent (`self.UseBlackboard` "/Game/Dynamic/Character/AI/PatrolData.PatrolData"))
  (`self.RunBehaviorTree` "/Game/Dynamic/Character/AI/GuardBehaviour.GuardBehaviour")
  (set `self.BlackboardComp` _blackboardcomponent))

(event `self.AIPerception.OnTargetPerceptionUpdated`
  (params (Actor :type "Actor Object Reference") (Stimulus :type "AIStimulus Structure"))
  (bind _enemykey (`self.EnemyKey`))
  (bind _blackboardcomp (`self.BlackboardComp`))
  ;[1 1 1] Update blackboard enemy key
  (if (`self.ActorHasTag` Actor "Enemy")
    _
    (elif (`.bSuccessfullySensed` (break `AIStimulus` Stimulus))
      (`BlackboardComponent.SetValueAsObject` _blackboardcomp _enemykey Actor)
      (else
        (`BlackboardComponent.ClearValue` _blackboardcomp _enemykey)))))

(fn `FindPatrolRoute`
  (params (Blackboard :type "BlackboardComponent Object Reference")))

(fn `UserConstructionScript`)