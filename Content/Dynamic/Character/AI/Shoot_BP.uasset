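; Behavior tree task that makes an AI-controlled Ue4ASP_Character aim and shoot at its target.
; On execute it sets the pawn's Aiming and Shooting flags and focuses the controller on the blackboard Target actor.
; It never finishes execution itself, so it runs until aborted, when it clears both flags and the focus, then finishes the abort.
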(event `self.ReceiveExecuteAI`
  (params (OwnerController :type "AIController Object Reference") (ControlledPawn :type "Pawn Object Reference"))
  (bind _asue_4asp_character (cast `/Game/Dynamic/Character/Behaviour/Ue4ASP_Character` ControlledPawn))
  (set `/Game/Dynamic/Character/Behaviour/Ue4ASP_Character.Aiming` true _asue_4asp_character)
  (set `/Game/Dynamic/Character/Behaviour/Ue4ASP_Character.Shooting` true _asue_4asp_character)
  (`AIController.K2_SetFocus` OwnerController (`BTFunctionLibrary.GetBlackboardValueAsActor` (`self.Target`))))

(event `self.ReceiveAbortAI`
  (params (OwnerController :type "AIController Object Reference") (ControlledPawn :type "Pawn Object Reference"))
  (bind _asue_4asp_character (cast `/Game/Dynamic/Character/Behaviour/Ue4ASP_Character` ControlledPawn))
  (set `/Game/Dynamic/Character/Behaviour/Ue4ASP_Character.Aiming` false _asue_4asp_character)
  (set `/Game/Dynamic/Character/Behaviour/Ue4ASP_Character.Shooting` false _asue_4asp_character)
  (`AIController.K2_ClearFocus` OwnerController)
  (`self.FinishAbort`))