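; Player character Blueprint that handles damage, death, pausing and landing noise.
; Damage plays a post-process fade timeline and reduces Health; at zero the character is unpossessed and the view blends to a spawned death camera, using the controller cached on possession.
; The 1 key opens the pause widget and pauses the game, and landing reports a noise event.
; The delayed game-over screen logic exists but is never run.
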(event `Key|One`
  (params (Key :type "Key Structure"))
  (:`Pressed`
    (if (not (`self.isPaused`))
      (bind _returnvalue (`|CreateWidget` "/Game/Dynamic/Character/UI/WBP_Pause.WBP_Pause_C"))
      (`UserWidget.AddToViewport` _returnvalue 0)
      (set `PlayerController.bShowMouseCursor` true (`GameplayStatics.GetPlayerController` 0))
      (set `self.isPaused` true)
      (`GameplayStatics.SetGamePaused` true))))

(event `self.OnLanded`
  (params (Hit :type "HitResult Structure (by ref)"))
  (`AISense_Hearing.ReportNoiseEvent` (`self.K2_GetActorLocation`) 1.0 self))

(event `self.ReceiveAnyDamage`
  (params (Damage :type "Float (single-precision)") (DamageType :type "DamageType Object Reference") (InstigatedBy :type "Controller Object Reference") (DamageCauser :type "Actor Object Reference"))
  (`|ExecutionSequence`
    (:`then_0`
      (bind (_direction _blend_weight) (`Timeline|DamageFade` :!via `PlayFromStart`)
        (:`Update`
          (set `PostProcessComponent.BlendWeight` _blend_weight (`self.PostProcess`)))))
    (:`then_1`
      (`self.TakeDamage` Damage))))

(event `self.ReceivePossessed`
  (params (NewController :type "Controller Object Reference"))
  (bind _output_get (set `self.OldController` NewController))
  (bind _asplayer_controller (cast `PlayerController` _output_get))
  (`PlayerController.SetViewTargetWithBlend` _asplayer_controller self 0.0 "VTBlend_Linear" 0.0 false))

(fn `IsDead`
  (returns (Dead :type Boolean))
  (return (<= (`self.Health`) 0.0)))

(fn `KillCharacter`
  (`Controller.UnPossess` (`self.GetController`))
  (`self.SpawnDeathCamera`))

(fn `SpawnDeathCamera`
  (bind _asplayer_controller (cast `PlayerController` (`self.OldController`)))
  (cast `CameraActor` (`Controller.GetViewTarget` _asplayer_controller)
    (:`CastFailed`
      (bind _returnvalue (`|SpawnActorFromClass` "/Script/Engine.CameraActor" (`SceneComponent.K2_GetComponentToWorld` (`self.DeathCameraSpawnPoint`)) "Undefined" "OverrideRootScale" null null))
      (`PlayerController.SetViewTargetWithBlend` _asplayer_controller _returnvalue 1.0 "VTBlend_Linear" 0.0 false))))

(fn `TakeDamage`
  (params (Damage :type "Float (double-precision)"))
  (set `self.Health` (- (`self.Health`) Damage))
  (bind _dead (`self.IsDead`))
  (if _dead
    (`self.KillCharacter`)))

(fn `UserConstructionScript`)