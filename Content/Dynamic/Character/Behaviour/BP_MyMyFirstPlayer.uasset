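; BP_MyMyFirstPlayer is a player character Blueprint with basic health and noise reporting.
; Landing reports a noise event at the character's location with itself as instigator, so AI can hear it.
; Any damage subtracts from Health, and once IsDead finds it at zero or below, the character detaches from its controller pending destruction.
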(event `self.OnLanded`
  (params (Hit :type "HitResult Structure (by ref)"))
  (`AISense_Hearing.ReportNoiseEvent` (`self.K2_GetActorLocation`) 1.0 self))

(event `self.ReceiveAnyDamage`
  (params (Damage :type "Float (single-precision)") (DamageType :type "DamageType Object Reference") (InstigatedBy :type "Controller Object Reference") (DamageCauser :type "Actor Object Reference"))
  (set `self.Health` (- (`self.Health`) Damage))
  (bind _dead (`self.IsDead`))
  (if _dead
    (`self.DetachFromControllerPendingDestroy`)))

(fn `IsDead`
  (returns (Dead :type Boolean))
  (return (<= (`self.Health`) 0.0)))

(fn `UserConstructionScript`)